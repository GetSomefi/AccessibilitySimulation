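; PlayerHUD creates the player's HUD widget on BeginPlay and drives its mission display and feedback animations.
; Each Tick polls flags: GoodJob and GainedScore each play their widget animation, then clear themselves and reset their DoOnce gate for reuse.
; While ShowMission is true, Tick rewrites header and description from arrays indexed by CurrentMission, playing the mission box animation through a DoOnce that is never reset here.
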(event `self.ReceiveBeginPlay`
  (bind _returnvalue (`|CreateWidget` "/Game/Blueprints/PlayerHUDWidget.PlayerHUDWidget_C"))
  (`UserWidget.AddToViewport` _returnvalue 0))

(event `self.ReceiveTick`
  (params (DeltaSeconds :type "Float (single-precision)"))
  (bind _currentmission (`self.CurrentMission`))
  (`|ExecutionSequence`
    (:`then_0`
      (if (`self.GoodJob`)
        (`/Engine/EditorBlueprintResources/StandardMacros.DoOnce` false :!label _label
          (:`Completed`
            (`UserWidget.PlayAnimation` (stale `self.ReceiveBeginPlay` _returnvalue) (`/Game/Blueprints/PlayerHUDWidget.GoodJob` (stale `self.ReceiveBeginPlay` _returnvalue)) 0.0 1 "Forward" 0.5)
            (set `self.GoodJob` false)
            (goto _label :!via `Reset`)))))
    (:`then_1`
      (if (`self.ShowMission`)
        (`TextBlock.SetText` (`/Game/Blueprints/PlayerHUDWidget.MissionHeader` (stale `self.ReceiveBeginPlay` _returnvalue)) (`KismetArrayLibrary.Array_Get` (`self.MissionHeaders`) _currentmission))
        (`TextBlock.SetText` (`/Game/Blueprints/PlayerHUDWidget.MissionText` (stale `self.ReceiveBeginPlay` _returnvalue)) (`KismetArrayLibrary.Array_Get` (`self.MissionDescriptions`) _currentmission))
        (`/Engine/EditorBlueprintResources/StandardMacros.DoOnce` false
          (:`Completed`
            (`UserWidget.PlayAnimation` (stale `self.ReceiveBeginPlay` _returnvalue) (`/Game/Blueprints/PlayerHUDWidget.MissionBoxAnim` (stale `self.ReceiveBeginPlay` _returnvalue)) 0.0 1 "Forward" 1.0)
            (`UserWidget.PlayAnimation` (stale `self.ReceiveBeginPlay` _returnvalue) (`/Game/Blueprints/PlayerHUDWidget.MissionBoxAnim` (stale `self.ReceiveBeginPlay` _returnvalue)) 0.0 1 "Forward" 1.0)))))
    (:`then_2`
      (if (`self.GainedScore`)
        (`/Engine/EditorBlueprintResources/StandardMacros.DoOnce` false :!label _label_2
          (:`Completed`
            (`UserWidget.PlayAnimation` (stale `self.ReceiveBeginPlay` _returnvalue) (`/Game/Blueprints/PlayerHUDWidget.GainedScore` (stale `self.ReceiveBeginPlay` _returnvalue)) 0.0 1 "Forward" 1.0)
            (set `self.GainedScore` false)
            (goto _label_2 :!via `Reset`)))))))

(fn `UserConstructionScript`)