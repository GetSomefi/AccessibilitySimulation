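; Player pawn with look and move input, an action key, and scoring of barrier and accessibility points.
; MasterOverlap contacts add barrier points and block forward movement and yaw until the overlap ends.
; Each tick, a short camera line trace is matched to FrontDescNPC by string comparison, toggling its talk board.
; Holding action on its Q1 option activates that stage, with a one-time HUD reward and accessibility point.
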(event `InputAction|ActionKey`
  (params (Key :type "Key Structure" :default "AnyKey"))
  ;[1 1 1] GrabAndAction
  (:`Pressed`
    (set `self.Grabing` true)
    (set `self.Action` true))
  (:`Released`
    (set `self.Grabing` false)
    (set `self.Action` false)))

(event `InputAxis|Look_R_L`
  (params (AxisValue :type "Float (single-precision)"))
  ;[1 1 1] RightToLeft
  (if (not (`self.IsOverlapping`))
    (`self.AddControllerYawInput` AxisValue)))

(event `InputAxis|Look_U_D`
  (params (AxisValue :type "Float (single-precision)"))
  ;[1 1 1] UpAndDown
  (`self.AddControllerPitchInput` AxisValue))

(event `InputAxis|MoveForwardKey`
  (params (AxisValue :type "Float (single-precision)"))
  ;[1 1 1] Left Right
  (if (not (`self.IsOverlapping`))
    (`self.AddMovementInput` (`KismetMathLibrary.GetForwardVector` (`self.GetControlRotation`)) AxisValue)))

(event `InputAxis|TurnKey`
  (params (AxisValue :type "Float (single-precision)"))
  ;[1 1 1] Left Right
  (`self.AddMovementInput` (`KismetMathLibrary.GetRightVector` (`self.GetControlRotation`)) AxisValue))

(event `self.MasterOverlap.OnComponentBeginOverlap`
  (params (OverlappedComponent :type "PrimitiveComponent Object Reference") (OtherActor :type "Actor Object Reference") (OtherComp :type "PrimitiveComponent Object Reference") (OtherBodyIndex :type Integer) (bFromSweep :type Boolean) (SweepResult :type "HitResult Structure (by ref)"))
  ;[1 1 1] Overlap protection
  (`KismetSystemLibrary.PrintString` "overlap")
  (`KismetSystemLibrary.PrintString` (`KismetStringLibrary.Conv_ObjectToString` OtherActor))
  (`KismetSystemLibrary.PrintString` (`KismetStringLibrary.Conv_ObjectToString` OverlappedComponent))
  (set `self.IsOverlapping` true)
  (bind _result (`/Engine/EditorBlueprintResources/StandardMacros.IncrementInt` (`self.BarrierPoints`))
    (:`  `
      (set `self.BarrierPoints` _result))))

(event `self.MasterOverlap.OnComponentEndOverlap`
  (params (OverlappedComponent :type "PrimitiveComponent Object Reference") (OtherActor :type "Actor Object Reference") (OtherComp :type "PrimitiveComponent Object Reference") (OtherBodyIndex :type Integer))
  ;[1 1 1] Overlap protection
  (`KismetSystemLibrary.PrintString` "overlap end")
  (set `self.IsOverlapping` false))

(event `self.ReceiveTick`
  (params (DeltaSeconds :type "Float (single-precision)"))
  (bind _returnvalue (`GameplayStatics.GetPlayerCameraManager` 0))
  (bind _returnvalue_2 (`PlayerCameraManager.GetCameraLocation` _returnvalue))
  ;[1 1 1] Players vision
  (bind _outhit (`KismetSystemLibrary.LineTraceSingle` :`Start` _returnvalue_2 :`End` (+ _returnvalue_2 (* (`KismetMathLibrary.GetForwardVector` (`self.K2_GetActorRotation` _returnvalue)) 200)) :`TraceChannel` "TraceTypeQuery1" :`DrawDebugType` "ForOneFrame"))
  (`|ExecutionSequence`
    (:`then_0`
      (bind (_bblockinghit _binitialoverlap _time _location _impactpoint _normal _impactnormal _physmat _hitactor _hitcomponent) (`GameplayStatics.BreakHitResult` _outhit))
      (bind _outactors (`GameplayStatics.GetAllActorsOfClass` (`GameplayStatics.GetObjectClass` _hitactor)))
      (for _array_element _outactors
        _)
      (if (== (`KismetStringLibrary.Conv_ObjectToString` (stale _array_element_3)) (`KismetStringLibrary.Conv_ObjectToString` _array_element))
        (`|ExecutionSequence`
          (:`then_0`
            (bind _asfront_desc_npc (cast `/Game/Blueprints/FrontDescNPC` _array_element))
            (`|ExecutionSequence`
              (:`then_0`
                (`/Engine/EditorBlueprintResources/StandardMacros.DoOnce` false
                  (:`Completed`
                    (`KismetSystemLibrary.PrintString` (`KismetTextLibrary.Conv_TextToString` (`/Game/Blueprints/FrontDescNPC.Hello` _asfront_desc_npc))))))
              (:`then_1`
                (if (== (`KismetStringLibrary.Conv_ObjectToString` (`/Game/Blueprints/FrontDescNPC.q1` _asfront_desc_npc)) (`KismetStringLibrary.Conv_ObjectToString` (`SceneComponent.GetChildComponent` _hitcomponent 0)))
                  (if (`self.Action`)
                    (set `/Game/Blueprints/FrontDescNPC.q1Stage` true _asfront_desc_npc)
                    (`KismetSystemLibrary.PrintString` "Q1 active")
                    (`/Engine/EditorBlueprintResources/StandardMacros.DoOnce` false
                      (:`Completed`
                        (bind _asplayer_hud (cast `/Game/Blueprints/PlayerHUD` (`PlayerController.GetHUD` (`GameplayStatics.GetPlayerController` 0))))
                        (set `/Game/Blueprints/PlayerHUD.GoodJob` true _asplayer_hud)
                        (set `/Game/Blueprints/PlayerHUD.GainedScore` true _asplayer_hud)
                        (set `self.AccessibilityPoints` (+ (`self.AccessibilityPoints`) 1)))))))))
          (:`then_1`
            (bind _asfront_desc_npc_2 (cast `/Game/Blueprints/FrontDescNPC` _array_element))
            (set `/Game/Blueprints/FrontDescNPC.TalkBoardOn` true _asfront_desc_npc_2)))
        (else
          (bind _outactors_2 (`GameplayStatics.GetAllActorsOfClass` "/Game/Blueprints/FrontDescNPC.FrontDescNPC_C"))
          (for _array_element_2 _outactors_2
            _)
          (set `/Game/Blueprints/FrontDescNPC.TalkBoardOn` false _array_element_2))))
    (:`then_1`
      (bind _outactors_3 (`GameplayStatics.GetAllActorsOfClass` "/Game/Blueprints/FrontDescNPC.FrontDescNPC_C"))
      (for _array_element_3 _outactors_3
        _))))

(fn `UserConstructionScript`)