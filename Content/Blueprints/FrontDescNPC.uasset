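; Front desk NPC Blueprint that unlocks the front doors based on a quest stage flag and shows or hides a talk board.
; While Q1Stage is true, Tick looks up the left and right opening doors by class, keeps them open and disables the front door trigger box, repeating this every frame.
; Tick also scales the text plane to full size or zero according to TalkBoardOn.
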(event `self.ReceiveTick`
  (params (DeltaSeconds :type "Float (single-precision)"))
  (`|ExecutionSequence`
    (:`then_0`
      (if (`self.q1Stage`)
        (`|ExecutionSequence`
          (:`then_0`
            (bind _outactors (`GameplayStatics.GetAllActorsOfClass` "/Game/Freebie_01/Meshes/OpeningDoorLeft.OpeningDoorLeft_C"))
            (set `/Game/Freebie_01/Meshes/OpeningDoorLeft.KeepDoorsOpen` true (`KismetArrayLibrary.Array_Get` _outactors)))
          (:`then_1`
            (bind _outactors_2 (`GameplayStatics.GetAllActorsOfClass` "/Game/Freebie_01/Meshes/OpeningDoorRight2.OpeningDoorRight2_C"))
            (set `/Game/Freebie_01/Meshes/OpeningDoorRight2.KeepDoorsOpen` true (`KismetArrayLibrary.Array_Get` _outactors_2))))
        (bind _outactors_3 (`GameplayStatics.GetAllActorsOfClass` "/Game/FrontDoorTriggerBox_Blueprint.FrontDoorTriggerBox_Blueprint_C"))
        (set `/Game/FrontDoorTriggerBox_Blueprint.Disabled` true (`KismetArrayLibrary.Array_Get` _outactors_3))))
    (:`then_1`
      (if (`self.TalkBoardOn`)
        (`SceneComponent.SetRelativeScale3D` (`self.PlaneForText`) (1.0 1.0 1.0))
        (else
          (`SceneComponent.SetRelativeScale3D` (`self.PlaneForText`) (0.0 0.0 0.0)))))))

(fn `UserConstructionScript`)